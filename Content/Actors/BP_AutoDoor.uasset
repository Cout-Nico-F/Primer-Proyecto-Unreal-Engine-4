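; BP_AutoDoor is an automatic door that slides a stone mesh while something overlaps its proximity trigger.
; Overlap begin plays a timeline that lerps the mesh's relative X from DoorStart to an offset, and overlap end reverses it.
; The construction script fills DoorStart from the mesh's relative Y, although the lerp drives X.
; A flag limits the music cue at the door to the first overlap.
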(event `self.Proximity_Trigger.OnComponentBeginOverlap`
  (params (OverlappedComponent :type "PrimitiveComponent Object Reference") (OtherActor :type "Actor Object Reference") (OtherComp :type "PrimitiveComponent Object Reference") (OtherBodyIndex :type Integer) (bFromSweep :type Boolean) (SweepResult :type "HitResult Structure (by ref)"))
  (bind _doorstart (`self.DoorStart`))
  (bind _sm_stone_05 (`self.SM_stone_05`))
  (bind _returnvalue (`SceneComponent.GetRelativeTransform` _sm_stone_05))
  (if (`self.AlreadyPlayed`)
    (bind (_direction _newtrack_0) (`Timeline|Timeline_0` :!label _label)
      (:`Update`
        (`SceneComponent.K2_SetRelativeLocation` _sm_stone_05 (`KismetMathLibrary.MakeVector` (`KismetMathLibrary.Lerp` _doorstart (- _doorstart 120.0) _newtrack_0) (.y (.location _returnvalue)) (.z (.location _returnvalue))) false false)))
    (else
      (set `self.AlreadyPlayed` true)
      (`GameplayStatics.PlaySoundAtLocation` "/Game/Audio/Starter_Music01.Starter_Music01" (`SceneComponent.K2_GetComponentLocation` _sm_stone_05) (struct) 1.0 1.0 0.0 null null null)
      (goto _label))))

(event `self.Proximity_Trigger.OnComponentEndOverlap`
  (params (OverlappedComponent :type "PrimitiveComponent Object Reference") (OtherActor :type "Actor Object Reference") (OtherComp :type "PrimitiveComponent Object Reference") (OtherBodyIndex :type Integer))
  (goto _label :!via `Reverse`))

(fn `UserConstructionScript`
  (set `self.DoorStart` (.y (.location (`SceneComponent.GetRelativeTransform` (`self.SM_stone_05`))))))